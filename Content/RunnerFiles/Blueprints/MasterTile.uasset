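; Endless runner track tile that fills its three lanes with random content and chains the track onward.
; On BeginPlay each lane makes successive independent random rolls for a pipe, box (capped at two per tile), coin or magnet; only the middle can spawn boots.
; When the player character overlaps its Box trigger, it has the GameMode spawn another tile, adds points, raises walk speed within limits, then destroys itself after a short delay.
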(event `self.ReceiveBeginPlay`
  (`self.SpawnObstaclesMiddle`)
  (`self.SpawnObstaclesLeft`)
  (`self.SpawnObstaclesRight`))

(event `self.Box.OnComponentBeginOverlap`
  (params (OverlappedComponent :type "PrimitiveComponent Object Reference") (OtherActor :type "Actor Object Reference") (OtherComp :type "PrimitiveComponent Object Reference") (OtherBodyIndex :type Integer) (bFromSweep :type Boolean) (SweepResult :type "HitResult Structure (by ref)"))
  (cast `/Game/ThirdPersonBP/Blueprints/ThirdPersonCharacter` OtherActor)
  (bind _asthird_person_game_mode (cast `/Game/ThirdPersonBP/Blueprints/ThirdPersonGameMode` (`GameplayStatics.GetGameMode`)))
  (`/Game/ThirdPersonBP/Blueprints/ThirdPersonGameMode.SpawnTile` _asthird_person_game_mode)
  (bind _asthird_person_game_mode_2 (cast `/Game/ThirdPersonBP/Blueprints/ThirdPersonGameMode` (`GameplayStatics.GetGameMode`)))
  (set `/Game/ThirdPersonBP/Blueprints/ThirdPersonGameMode.CurrentPoints` (+ (`/Game/ThirdPersonBP/Blueprints/ThirdPersonGameMode.CurrentPoints` _asthird_person_game_mode_2) (* (`/Game/ThirdPersonBP/Blueprints/ThirdPersonGameMode.PointMultiplier` _asthird_person_game_mode_2) 1)) _asthird_person_game_mode_2)
  (bind _asthird_person_character (cast `/Game/ThirdPersonBP/Blueprints/ThirdPersonCharacter` (`GameplayStatics.GetPlayerCharacter` 0)))
  (bind _charactermovement (`Character.CharacterMovement` _asthird_person_character))
  (set `CharacterMovementComponent.MaxWalkSpeed` (`KismetMathLibrary.FClamp` (* (`CharacterMovementComponent.MaxWalkSpeed` _charactermovement) 1.1) 600.0 1200.0) _charactermovement)
  (`KismetSystemLibrary.Delay` 0.5)
  (`self.K2_DestroyActor`))

(fn `SpawnObstaclesLeft`
  (bind _returnvalue (`KismetMathLibrary.RandomFloatInRange` 0.0 1.0))
  (bind _returnvalue_2 (`SceneComponent.K2_GetComponentToWorld` (`self.LeftLaneMid`)))
  ;[1 1 1] Left Lane Obstacles
  (if (`KismetMathLibrary.InRange_FloatFloat` _returnvalue 0.1 0.3)
    (`|SpawnActorFromClass` "/Game/RunnerFiles/Blueprints/Pipe_Blueprint.Pipe_Blueprint_C" _returnvalue_2 "Undefined" "OverrideRootScale" null null)
    (elif (`KismetMathLibrary.InRange_FloatFloat` _returnvalue 0.4 0.5)
      (if (not (>= (`self.BoxCount`) 2))
        (`|SpawnActorFromClass` "/Game/RunnerFiles/Blueprints/Box_Blueprint.Box_Blueprint_C" _returnvalue_2 "Undefined" "OverrideRootScale" null null)
        (set `self.BoxCount` (+ (`self.BoxCount`) 1)))
      (elif (`KismetMathLibrary.InRange_FloatFloat` _returnvalue 0.5 0.9)
        (`|SpawnActorFromClass` "/Game/RunnerFiles/Blueprints/Coin_Pickup.Coin_Pickup_C" _returnvalue_2 "Undefined" "OverrideRootScale" null null)
        (elif (`KismetMathLibrary.InRange_FloatFloat` _returnvalue 0.9 0.95)
          (`|SpawnActorFromClass` "/Game/RunnerFiles/Blueprints/Magnet_Pickup.Magnet_Pickup_C" _returnvalue_2 "Undefined" "OverrideRootScale" null null))))))

(fn `SpawnObstaclesMiddle`
  (bind _returnvalue (`KismetMathLibrary.RandomFloatInRange` 0.0 1.0))
  (bind _returnvalue_2 (`SceneComponent.K2_GetComponentToWorld` (`self.MidLaneMid`)))
  ;[1 1 1] Middle Lane Obstacles
  (if (`KismetMathLibrary.InRange_FloatFloat` _returnvalue 0.1 0.3)
    (`|SpawnActorFromClass` "/Game/RunnerFiles/Blueprints/Pipe_Blueprint.Pipe_Blueprint_C" _returnvalue_2 "Undefined" "OverrideRootScale" null null)
    (elif (`KismetMathLibrary.InRange_FloatFloat` _returnvalue 0.4 0.5)
      (if (not (>= (`self.BoxCount`) 2))
        (`|SpawnActorFromClass` "/Game/RunnerFiles/Blueprints/Box_Blueprint.Box_Blueprint_C" _returnvalue_2 "Undefined" "OverrideRootScale" null null)
        (set `self.BoxCount` (+ (`self.BoxCount`) 1)))
      (elif (`KismetMathLibrary.InRange_FloatFloat` _returnvalue 0.5 0.9)
        (`|SpawnActorFromClass` "/Game/RunnerFiles/Blueprints/Coin_Pickup.Coin_Pickup_C" _returnvalue_2 "Undefined" "OverrideRootScale" null null)
        (elif (`KismetMathLibrary.InRange_FloatFloat` _returnvalue 0.9 0.95)
          (`|SpawnActorFromClass` "/Game/RunnerFiles/Blueprints/Magnet_Pickup.Magnet_Pickup_C" _returnvalue_2 "Undefined" "OverrideRootScale" null null)
          (elif (`KismetMathLibrary.InRange_FloatFloat` _returnvalue 0.95)
            (`|SpawnActorFromClass` "/Game/RunnerFiles/Blueprints/Boot_Pickup.Boot_Pickup_C" _returnvalue_2 "Undefined" "OverrideRootScale" null null)))))))

(fn `SpawnObstaclesRight`
  (bind _returnvalue (`KismetMathLibrary.RandomFloatInRange` 0.0 1.0))
  (bind _returnvalue_2 (`SceneComponent.K2_GetComponentToWorld` (`self.RightLaneMid`)))
  ;[1 1 1] Right Lane Obstacles
  (if (`KismetMathLibrary.InRange_FloatFloat` _returnvalue 0.1 0.3)
    (`|SpawnActorFromClass` "/Game/RunnerFiles/Blueprints/Pipe_Blueprint.Pipe_Blueprint_C" _returnvalue_2 "Undefined" "OverrideRootScale" null null)
    (elif (`KismetMathLibrary.InRange_FloatFloat` _returnvalue 0.4 0.5)
      (if (not (>= (`self.BoxCount`) 2))
        (`|SpawnActorFromClass` "/Game/RunnerFiles/Blueprints/Box_Blueprint.Box_Blueprint_C" _returnvalue_2 "Undefined" "OverrideRootScale" null null)
        (set `self.BoxCount` (+ (`self.BoxCount`) 1)))
      (elif (`KismetMathLibrary.InRange_FloatFloat` _returnvalue 0.5 0.9)
        (`|SpawnActorFromClass` "/Game/RunnerFiles/Blueprints/Coin_Pickup.Coin_Pickup_C" _returnvalue_2 "Undefined" "OverrideRootScale" null null)
        (elif (`KismetMathLibrary.InRange_FloatFloat` _returnvalue 0.9 0.95)
          (`|SpawnActorFromClass` "/Game/RunnerFiles/Blueprints/Magnet_Pickup.Magnet_Pickup_C" _returnvalue_2 "Undefined" "OverrideRootScale" null null))))))

(fn `UserConstructionScript`)