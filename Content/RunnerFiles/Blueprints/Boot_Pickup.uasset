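; Boot pickup for a runner game that temporarily boosts the player's jump height.
; Overlapping the mesh raises the ThirdPersonCharacter's JumpZVelocity and hides the mesh, then after a ten-second delay restores the normal jump value and destroys the actor.
; A separate MissedDestroy trigger destroys the actor fifteen seconds after the player passes through it, cleaning up missed pickups.
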(event `self.StaticMesh.OnComponentBeginOverlap`
  (params (OverlappedComponent :type "PrimitiveComponent Object Reference") (OtherActor :type "Actor Object Reference") (OtherComp :type "PrimitiveComponent Object Reference") (OtherBodyIndex :type Integer) (bFromSweep :type Boolean) (SweepResult :type "HitResult Structure (by ref)"))
  (bind _asthird_person_character (cast `/Game/ThirdPersonBP/Blueprints/ThirdPersonCharacter` OtherActor))
  (set `CharacterMovementComponent.JumpZVelocity` 1200.0 (`Character.CharacterMovement` _asthird_person_character))
  (`SceneComponent.SetVisibility` (`self.StaticMesh`) false false)
  (`KismetSystemLibrary.Delay` 10.0)
  (bind _asthird_person_character_2 (cast `/Game/ThirdPersonBP/Blueprints/ThirdPersonCharacter` (`GameplayStatics.GetPlayerCharacter` 0)))
  (set `CharacterMovementComponent.JumpZVelocity` 600.0 (`Character.CharacterMovement` _asthird_person_character_2))
  (`self.K2_DestroyActor`))

(event `self.MissedDestroy.OnComponentBeginOverlap`
  (params (OverlappedComponent :type "PrimitiveComponent Object Reference") (OtherActor :type "Actor Object Reference") (OtherComp :type "PrimitiveComponent Object Reference") (OtherBodyIndex :type Integer) (bFromSweep :type Boolean) (SweepResult :type "HitResult Structure (by ref)"))
  (cast `/Game/ThirdPersonBP/Blueprints/ThirdPersonCharacter` OtherActor)
  (cast `/Game/ThirdPersonBP/Blueprints/ThirdPersonGameMode` (`GameplayStatics.GetGameMode`))
  (`KismetSystemLibrary.Delay` 15.0)
  (`self.K2_DestroyActor`))

(fn `UserConstructionScript`)